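; Drivable cyberpunk hover car that flies with gravity disabled on its physics body.
; Each tick adds yaw-relative throttle, steer and lift input to velocity, interpolates actor tilt and mouse-driven yaw, and banks the body mesh.
; LookRight is quantized into stepped turn rates through nested selects, while LookUp pitches the spring arm.
; Speed drives engine sound RPM and pitch; a debug PrintString of the turn value runs every tick.
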(event `self.ReceiveTick`
  (params (DeltaSeconds :type "Float (single-precision)"))
  (bind (_returnvalue_roll _returnvalue_pitch _returnvalue_yaw) (`KismetMathLibrary.BreakRotator` (`self.K2_GetActorRotation`)))
  (bind (_returnvalue_roll_2 _returnvalue_pitch_2 _returnvalue_yaw_2) (`KismetMathLibrary.BreakRotator` (`self.K2_GetActorRotation`)))
  (bind _returnvalue (`self.GetInputAxisValue`))
  (bind _sc_enginesound (`self.SC_EngineSound`))
  (bind _forward_speed (`self.Forward Speed`))
  (bind _returnvalue_2 (/ (`self.Get Up Speed`) 10.0))
  (bind _returnvalue_3 (* (`self.MouseRot`) (`self.Drone Horizontal Rotation`)))
  (bind (_returnvalue_roll_3 _returnvalue_pitch_3) (`KismetMathLibrary.BreakRotator` (`KismetMathLibrary.MakeRotator` (* (`self.GetInputAxisValue`) 10.0) (* (`self.GetInputAxisValue`) 10.0))))
  (bind _returnvalue_4 (`KismetMathLibrary.Abs` (`KismetMathLibrary.VSize` (`self.GetVelocity`))))
  (bind (_returnvalue_roll_4 _returnvalue_pitch_4 _returnvalue_yaw_3) (`KismetMathLibrary.BreakRotator` (`KismetMathLibrary.RInterpTo` (`KismetMathLibrary.MakeRotator` _returnvalue_roll _returnvalue_pitch _returnvalue_yaw) (`KismetMathLibrary.MakeRotator` _returnvalue_roll_3 _returnvalue_pitch_3 (+ _returnvalue_yaw _returnvalue_3)) (`self.Delta seconds`) 1.0)))
  (set `self.Delta seconds` DeltaSeconds)
  (`PrimitiveComponent.SetEnableGravity` (`self.plane`) false)
  (`PrimitiveComponent.SetPhysicsLinearVelocity` (`self.plane`) (+ (`self.GetVelocity`) (* (* (`KismetMathLibrary.GreaterGreater_VectorRotator` (`KismetMathLibrary.MakeVector` (* (`self.GetInputAxisValue`) _forward_speed -1.0) (* (`self.GetInputAxisValue`) _forward_speed) (`KismetMathLibrary.SelectFloat` (* _returnvalue_2 -1.0) (* _returnvalue _returnvalue_2) (== _returnvalue -1.0))) (`KismetMathLibrary.MakeRotator` 0.0 0.0 _returnvalue_yaw_2)) (`self.Movement speed`)) (`self.Delta seconds`))) false "None")
  (`KismetSystemLibrary.PrintString` (`KismetStringLibrary.Conv_DoubleToString` _returnvalue_3))
  (`self.K2_SetActorRotation` (`KismetMathLibrary.MakeRotator` _returnvalue_roll_4 _returnvalue_pitch_4 _returnvalue_yaw_3)) ; Rotate the helicopter yaw to match the camera, while pitch and roll are determined by input direction
  (bind _output_get (set `self.MouseRotRotation` (`KismetMathLibrary.FInterpTo` (`self.MouseRotRotation`) (* (`self.MouseRot`) 35.0) (`self.Delta seconds`) 2.0)))
  (bind _output_get_2 (set `self.SteerRotation` (`KismetMathLibrary.FInterpTo` (`self.SteerRotation`) (* (`self.GetInputAxisValue`) 20.0) (`self.Delta seconds`) 2.0)))
  (bind _returnvalue_5 (+ _output_get _output_get_2))
  (`SceneComponent.K2_SetRelativeRotation` (`self.Body`) (`KismetMathLibrary.MakeRotator` _returnvalue_5 0.0 (+ _returnvalue_5 90.0)) false false)
  (`AudioComponent.SetFloatParameter` _sc_enginesound "RPM" _returnvalue_4)
  (`AudioComponent.SetPitchMultiplier` _sc_enginesound (* (+ (/ _returnvalue_4 9000.0) 0.2) 5.0)))

(event `InputAxis|LookRight`
  (params (AxisValue :type "Float (single-precision)"))
  (set `self.MouseRot` (`KismetMathLibrary.SelectFloat` (`KismetMathLibrary.SelectFloat` (`KismetMathLibrary.SelectFloat` (`KismetMathLibrary.SelectFloat` (`KismetMathLibrary.SelectFloat` (`KismetMathLibrary.SelectFloat` (`KismetMathLibrary.SelectFloat` 0.7 0.6 (> AxisValue 0.6)) 0.4 (> AxisValue 0.5)) 0.4 (> AxisValue 0.4)) 0.3 (> AxisValue 0.3)) 0.2 (> AxisValue 0.2)) 0.1 (> AxisValue 0.1)) (`KismetMathLibrary.SelectFloat` (`KismetMathLibrary.SelectFloat` (`KismetMathLibrary.SelectFloat` (`KismetMathLibrary.SelectFloat` (`KismetMathLibrary.SelectFloat` (`KismetMathLibrary.SelectFloat` (`KismetMathLibrary.SelectFloat` -0.7 -0.6 (< AxisValue -0.6)) -0.5 (< AxisValue -0.5)) -0.4 (< AxisValue -0.4)) -0.3 (< AxisValue -0.3)) -0.2 (< AxisValue -0.2)) -0.1 (< AxisValue -0.1)) 0.0 (< AxisValue 0.0)) (> AxisValue 0.0))))

(event `InputAxis|LookUp`
  (params (AxisValue :type "Float (single-precision)"))
  (`SceneComponent.K2_AddRelativeRotation` (`self.SpringArm`) (`KismetMathLibrary.MakeRotator` 0.0 AxisValue) false false))

(fn `UserConstructionScript`)