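; BP_CR01Hover is a component that provides hover suspension for the BP_CR01Drivable car that owns it.
; Each tick it traces down its own up vector to measure how far it sits inside the hover distance.
; A spring-damper turns that compression and its rate of change into a force on the car's root primitive at the component's location.
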(event `self.ReceiveBeginPlay`
  (bind _asbp_cr01drivable (cast `/Game/CyberPunkMegapack/Blueprints/Cars01/BP_CR01Drivable` (`self.GetOwner`)))
  (set `self.CyberpunkDragCar` _asbp_cr01drivable))

(event `self.ReceiveTick`
  (params (DeltaSeconds :type "Float (single-precision)"))
  (bind _returnvalue (`self.K2_GetComponentLocation`))
  (`/Engine/EditorBlueprintResources/StandardMacros.IsValid` (`self.CyberpunkDragCar`)
    (:`Is Valid`
      (bind (_outhit _returnvalue_2) (`KismetSystemLibrary.LineTraceSingle` _returnvalue (- _returnvalue (* (`self.GetUpVector`) (`self.Hover Distance`))) "TraceTypeQuery1"))
      (if _returnvalue_2
        (bind _output_get (set `self.Hover Delta` (- (`self.Hover Distance`) (`.Distance` (`GameplayStatics.BreakHitResult` _outhit)))))
        (`PrimitiveComponent.AddForceAtLocation` (cast `PrimitiveComponent` (`Actor.RootComponent` (`self.CyberpunkDragCar`)) :!pure true) (* (`self.GetUpVector`) (+ (* (/ (- _output_get (`self.PreviousHoverDelta`)) (`GameplayStatics.GetWorldDeltaSeconds`)) (`self.DampingCoefficient`)) (* _output_get (`self.SpringCoefficient`)))) (`self.K2_GetComponentLocation`) "None")
        (set `self.PreviousHoverDelta` (`self.Hover Delta`))))))