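; Drivable cyberpunk hover car with animated controls and doors, toggleable headlights, brake lights and speed-pitched engine audio.
; Tick turns throttle, steer and lift input into yaw-relative physics velocity on Plane, toggles its gravity by height, and interpolates banking and turning.
; Key flip-flops drive doors and headlights; Handbrake is inverted, false while Space is held, zeroing drive input.
; Construction script applies paint, dirt, edge wear and headlight color.
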(event `self.ReceiveTick`
  (params (DeltaSeconds :type "Float (single-precision)"))
  (bind (_returnvalue_roll _returnvalue_pitch _returnvalue_yaw) (`KismetMathLibrary.BreakRotator` (`self.K2_GetActorRotation`)))
  (bind (_returnvalue_roll_2 _returnvalue_pitch_2 _returnvalue_yaw_2) (`KismetMathLibrary.BreakRotator` (`self.K2_GetActorRotation`)))
  (bind _returnvalue (`self.GetInputAxisValue`))
  (bind _returnvalue_2 (`self.GetInputAxisValue`))
  (bind _returnvalue_3 (`self.GetInputAxisValue`))
  (bind _returnvalue_4 (`self.GetInputAxisValue`))
  (bind _plane (`self.plane`))
  (bind _sc_enginesound (`self.SC_EngineSound`))
  (bind _sc_doors_v (`self.SC_Doors_V`))
  (bind _frontlight_intensity (`self.FrontLight Intensity`))
  (bind _handbrake (`self.Handbrake`))
  (bind _returnvalue_5 (`KismetMathLibrary.Conv_BoolToDouble` _handbrake))
  (bind (_returnvalue_x _returnvalue_y _returnvalue_z) (`KismetMathLibrary.BreakVector` (`SceneComponent.K2_GetComponentLocation` _plane)))
  (bind _returnvalue_6 (`KismetMathLibrary.Conv_BoolToDouble` (`self.Frontlights`)))
  (bind _returnvalue_7 (`KismetMathLibrary.Abs` (`KismetMathLibrary.VSize` (`self.GetVelocity`))))
  (bind (_returnvalue_roll_3 _returnvalue_pitch_3) (`KismetMathLibrary.BreakRotator` (`KismetMathLibrary.MakeRotator` (* (`KismetMathLibrary.Conv_BoolToDouble` (`self.Handbrake`)) (+ (* _returnvalue_2 10.0) (* _returnvalue_3 15.0))) (* _returnvalue_2 30.0))))
  (bind (_returnvalue_roll_4 _returnvalue_pitch_4 _returnvalue_yaw_3) (`KismetMathLibrary.BreakRotator` (`KismetMathLibrary.RInterpTo` (`KismetMathLibrary.MakeRotator` _returnvalue_roll _returnvalue_pitch _returnvalue_yaw) (`KismetMathLibrary.MakeRotator` _returnvalue_roll_3 _returnvalue_pitch_3 (+ _returnvalue_yaw (* (* (`KismetMathLibrary.SelectFloat` -1.0 1.0 (== _returnvalue_3 -1.0)) (`self.GetInputAxisValue`)) (`self.Rotation Speed`)))) (`self.Delta seconds`) 1.0)))
  (bind _output_get (set `self.Speed` (`KismetMathLibrary.FInterpTo` (`self.Speed`) (* (* (`self.GetInputAxisValue`) _returnvalue_5) (`self.Forward Speed`) 0.05) DeltaSeconds 1.0)))
  (`PrimitiveComponent.SetEnableGravity` _plane (not (> _returnvalue_z 400.0)))
  (set `self.Delta seconds` DeltaSeconds)
  (`PrimitiveComponent.SetPhysicsLinearVelocity` (`self.plane`) (+ (`self.GetVelocity`) (* (* (`KismetMathLibrary.GreaterGreater_VectorRotator` (`KismetMathLibrary.MakeVector` (* (* (`self.GetInputAxisValue`) _returnvalue_5) (`self.Steer Push`) -0.05) (`KismetMathLibrary.SelectFloat` _output_get 0.0 _handbrake) (`KismetMathLibrary.SelectFloat` (* _returnvalue_5 _returnvalue) (* _returnvalue_5 _returnvalue 5.0) (== _returnvalue -1.0))) (`KismetMathLibrary.MakeRotator` 0.0 0.0 _returnvalue_yaw_2)) (`self.Movement speed`)) (`self.Delta seconds`))) false "None")
  (`self.K2_SetActorRotation` (`KismetMathLibrary.MakeRotator` _returnvalue_roll_4 _returnvalue_pitch_4 _returnvalue_yaw_3))
  (bind _output_get_2 (set `self.Acceleration Loc` (`KismetMathLibrary.FInterpTo` (`self.Acceleration Loc`) (* (`self.GetInputAxisValue`) 6.0) (`GameplayStatics.GetWorldDeltaSeconds`) 4.0)))
  (`SceneComponent.K2_SetRelativeLocation` (`self.accelerator`) (`KismetMathLibrary.MakeVector` 0.109192 (+ _output_get_2 31.5) 56.007511) false false)
  (bind _output_get_3 (set `self.SteeringWheelRot` (`KismetMathLibrary.FInterpTo` (`self.SteeringWheelRot`) (* _returnvalue_4 55.0) (`GameplayStatics.GetWorldDeltaSeconds`) 4.0)))
  (`SceneComponent.K2_SetRelativeRotation` (`self.SteeringWheel`) (`KismetMathLibrary.MakeRotator` 0.0 _output_get_3) false false)
  (bind _output_get_4 (set `self.WheelFL` (`KismetMathLibrary.FInterpTo` (`self.WheelFL`) (`KismetMathLibrary.SelectFloat` _returnvalue_4 0.0 (== _returnvalue_4 -1.0)) (`GameplayStatics.GetWorldDeltaSeconds`) 2.5)))
  (`SceneComponent.K2_SetRelativeLocationAndRotation` (`self.FL`) (`KismetMathLibrary.MakeVector` (+ (* _output_get_4 21.0) 101.353996) (+ (* _output_get_4 -7.0) 83.130997) (+ (* _output_get_4 -21.0) 38.422001)) (`KismetMathLibrary.MakeRotator` 0.0 (* _output_get_4 9.999983)) false false)
  (bind _output_get_5 (set `self.WheelFR` (`KismetMathLibrary.FInterpTo` (`self.WheelFR`) (`KismetMathLibrary.SelectFloat` _returnvalue_4 0.0 (== _returnvalue_4 1.0)) (`GameplayStatics.GetWorldDeltaSeconds`) 2.5)))
  (`SceneComponent.K2_SetRelativeLocationAndRotation` (`self.FR`) (`KismetMathLibrary.MakeVector` (+ (* _output_get_5 21.0) -101.353996) (+ (* _output_get_5 7.0) 83.130997) (+ (* _output_get_5 21.0) 38.422001)) (`KismetMathLibrary.MakeRotator` 0.0 (* _output_get_5 9.999983)) false false)
  (bind _output_get_6 (set `self.Left Door` (`KismetMathLibrary.FInterpTo` (`self.Left Door`) (`KismetMathLibrary.Conv_BoolToDouble` (`self.LeftDoor`)) (`GameplayStatics.GetWorldDeltaSeconds`) 2.5)))
  (bind _returnvalue_8 (* _output_get_6 60.0))
  (`SceneComponent.K2_SetRelativeRotation` (`self.DoorLeft`) (`KismetMathLibrary.MakeRotator` 0.0 0.0 _returnvalue_8) false false)
  (`AudioComponent.SetFloatParameter` _sc_doors_v "FLRot" _returnvalue_8)
  (`AudioComponent.SetBoolParameter` _sc_doors_v "DoorFL" (`self.LeftDoor`))
  (bind _output_get_7 (set `self.Right Door` (`KismetMathLibrary.FInterpTo` (`self.Right Door`) (`KismetMathLibrary.Conv_BoolToDouble` (`self.RightDoor`)) (`GameplayStatics.GetWorldDeltaSeconds`) 2.5)))
  (bind _returnvalue_9 (* _output_get_7 -60.0))
  (`SceneComponent.K2_SetRelativeRotation` (`self.DoorRight`) (`KismetMathLibrary.MakeRotator` 0.0 0.0 _returnvalue_9) false false)
  (`AudioComponent.SetFloatParameter` _sc_doors_v "FRRot" _returnvalue_9)
  (`AudioComponent.SetBoolParameter` _sc_doors_v "DoorFR" (`self.RightDoor`))
  (if (or (== (`self.Handbrake`) false) (== (`self.GetInputAxisValue`) -1.0))
    (set `self.stoplights` 300.0)
    (else
      (set `self.stoplights` 0.0)))
  (`LightComponent.SetIntensity` (`self.PointLight13`) (`self.stoplights`))
  (`LightComponent.SetIntensity` (`self.PointLight5`) (`self.stoplights`))
  (`LightComponent.SetIntensity` (`self.PointLight1`) (`self.stoplights`))
  (`LightComponent.SetIntensity` (`self.PointLight2`) (`self.stoplights`))
  (`LightComponent.SetIntensity` (`self.PointLight3`) (`self.stoplights`))
  (`LightComponent.SetIntensity` (`self.PointLight`) (`self.stoplights`))
  (`LightComponent.SetIntensity` (`self.FrontLight4`) (* _returnvalue_6 _frontlight_intensity))
  (`LightComponent.SetIntensity` (`self.FrontLight3`) (* _returnvalue_6 _frontlight_intensity))
  (`LightComponent.SetIntensity` (`self.FrontLight2`) (* _returnvalue_6 _frontlight_intensity))
  (`LightComponent.SetIntensity` (`self.FrontLight1`) (* _returnvalue_6 _frontlight_intensity))
  (`LightComponent.SetIntensity` (`self.SpotLight`) (* _returnvalue_6 (* _frontlight_intensity 800.0)))
  (`LightComponent.SetIntensity` (`self.SpotLight1`) (* _returnvalue_6 (* _frontlight_intensity 800.0)))
  (`AudioComponent.SetFloatParameter` _sc_enginesound "RPM" _returnvalue_7)
  (`AudioComponent.SetPitchMultiplier` _sc_enginesound (* (+ (/ _returnvalue_7 9000.0) 0.2) 3.0)))

(event `InputAxis|LookUp`
  (params (AxisValue :type "Float (single-precision)"))
  (`SceneComponent.K2_AddRelativeRotation` (`self.SpringArm`) (`KismetMathLibrary.MakeRotator` 0.0 AxisValue (stale `InputAxis|LookRight` AxisValue)) false false :!label _label))

(event `InputAxis|LookRight`
  (params (AxisValue :type "Float (single-precision)"))
  (goto _label))

(event `Key|R`
  (params (Key :type "Key Structure"))
  (:`Pressed`
    (bind _isa (`/Engine/EditorBlueprintResources/StandardMacros.FlipFlop`)
      (:`A`
        _)
      (:`B`
        _))
    (set `self.RightDoor` _isa)))

(event `Key|T`
  (params (Key :type "Key Structure"))
  (:`Pressed`
    (bind _isa (`/Engine/EditorBlueprintResources/StandardMacros.FlipFlop`)
      (:`A`
        _)
      (:`B`
        _))
    (set `self.Frontlights` _isa)))

(event `Key|F`
  (params (Key :type "Key Structure"))
  (:`Pressed`
    (bind _isa (`/Engine/EditorBlueprintResources/StandardMacros.FlipFlop`)
      (:`A`
        _)
      (:`B`
        _))
    (set `self.LeftDoor` _isa)))

(event `Key|SpaceBar`
  (params (Key :type "Key Structure"))
  (:`Pressed`
    (set `self.Handbrake` false))
  (:`Released`
    (set `self.Handbrake` true)))

(fn `UserConstructionScript`
  (bind _body (`self.Body`))
  (bind _dirt_level (`self.Dirt Level`))
  (`MeshComponent.SetVectorParameterValueOnMaterials` _body "CarPaint" (`KismetMathLibrary.Conv_LinearColorToVector` (`self.Body Color`)))
  (`MeshComponent.SetVectorParameterValueOnMaterials` (`self.DoorRight`) "CarPaint" (`KismetMathLibrary.Conv_LinearColorToVector` (`self.Body Color`)))
  (`MeshComponent.SetVectorParameterValueOnMaterials` (`self.DoorLeft`) "CarPaint" (`KismetMathLibrary.Conv_LinearColorToVector` (`self.Body Color`)))
  (`MeshComponent.SetVectorParameterValueOnMaterials` (`self.FR`) "CarPaint" (`KismetMathLibrary.Conv_LinearColorToVector` (`self.Body Color`)))
  (`MeshComponent.SetVectorParameterValueOnMaterials` (`self.FL`) "CarPaint" (`KismetMathLibrary.Conv_LinearColorToVector` (`self.Body Color`)))
  (`MeshComponent.SetVectorParameterValueOnMaterials` (`self.Exhaust`) "CarPaint" (`KismetMathLibrary.Conv_LinearColorToVector` (`self.Body Color`)))
  (`MeshComponent.SetScalarParameterValueOnMaterials` _body "DirtLayer" _dirt_level)
  (`MeshComponent.SetScalarParameterValueOnMaterials` (`self.DoorLeft`) "DirtLayer" _dirt_level)
  (`MeshComponent.SetScalarParameterValueOnMaterials` (`self.DoorRight`) "DirtLayer" _dirt_level)
  (`MeshComponent.SetScalarParameterValueOnMaterials` (`self.FR`) "DirtLayer" _dirt_level)
  (`MeshComponent.SetScalarParameterValueOnMaterials` (`self.FL`) "DirtLayer" _dirt_level)
  (`MeshComponent.SetScalarParameterValueOnMaterials` (`self.Exhaust`) "DirtLayer" _dirt_level)
  (`MeshComponent.SetScalarParameterValueOnMaterials` (`self.FL`) "DirtRoughness" (* _dirt_level 2.0))
  (`MeshComponent.SetScalarParameterValueOnMaterials` (`self.FR`) "DirtRoughness" (* _dirt_level 2.0))
  (`MeshComponent.SetScalarParameterValueOnMaterials` (`self.DoorRight`) "DirtRoughness" (* _dirt_level 2.0))
  (`MeshComponent.SetScalarParameterValueOnMaterials` (`self.DoorLeft`) "DirtRoughness" (* _dirt_level 2.0))
  (`MeshComponent.SetScalarParameterValueOnMaterials` _body "DirtRoughness" (* _dirt_level 2.0))
  (`MeshComponent.SetScalarParameterValueOnMaterials` (`self.Exhaust`) "DirtRoughness" (* _dirt_level 2.0))
  (`MeshComponent.SetScalarParameterValueOnMaterials` _body "TurnOn_EdgeWear" _dirt_level)
  (`MeshComponent.SetScalarParameterValueOnMaterials` (`self.DoorLeft`) "TurnOn_EdgeWear" _dirt_level)
  (`MeshComponent.SetScalarParameterValueOnMaterials` (`self.FR`) "TurnOn_EdgeWear" _dirt_level)
  (`MeshComponent.SetScalarParameterValueOnMaterials` (`self.FL`) "TurnOn_EdgeWear" _dirt_level)
  (`MeshComponent.SetScalarParameterValueOnMaterials` (`self.Exhaust`) "TurnOn_EdgeWear" _dirt_level)
  (`MeshComponent.SetScalarParameterValueOnMaterials` _body "EdgeWear_Contrast" (+ (* _dirt_level 20.0) 1.0))
  (`MeshComponent.SetScalarParameterValueOnMaterials` (`self.DoorRight`) "EdgeWear_Contrast" (+ (* _dirt_level 20.0) 1.0))
  (`MeshComponent.SetScalarParameterValueOnMaterials` (`self.DoorLeft`) "EdgeWear_Contrast" (+ (* _dirt_level 20.0) 1.0))
  (`MeshComponent.SetScalarParameterValueOnMaterials` (`self.FR`) "EdgeWear_Contrast" (+ (* _dirt_level 20.0) 1.0))
  (`MeshComponent.SetScalarParameterValueOnMaterials` (`self.FL`) "EdgeWear_Contrast" (+ (* _dirt_level 20.0) 1.0))
  (`MeshComponent.SetScalarParameterValueOnMaterials` (`self.Exhaust`) "EdgeWear_Contrast" (+ (* _dirt_level 20.0) 1.0))
  (`LightComponent.SetLightColor` (`self.SpotLight`) (`self.Front Light Color`) true)
  (`LightComponent.SetLightColor` (`self.SpotLight1`) (`self.Front Light Color`) true)
  (`LightComponent.SetLightColor` (`self.FrontLight3`) (`self.Front Light Color`) true)
  (`LightComponent.SetLightColor` (`self.FrontLight4`) (`self.Front Light Color`) true)
  (`LightComponent.SetLightColor` (`self.FrontLight2`) (`self.Front Light Color`) true)
  (`LightComponent.SetLightColor` (`self.FrontLight1`) (`self.Front Light Color`) true))