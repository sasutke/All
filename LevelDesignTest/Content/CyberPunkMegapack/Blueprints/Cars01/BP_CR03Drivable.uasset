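; Drivable flying hover car pawn with camera look, toggleable doors and headlights, and a space-bar handbrake.
; Tick turns throttle, steer and vertical input into physics velocity on Plane, disables its gravity above a height threshold, and interpolates banking and yaw.
; Tick also animates hover parts, doors and steering wheel, drives brake lights and headlights, and feeds door and speed-based engine audio.
; The construction script applies body color, dirt level and headlight color.
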(event `self.ReceiveTick`
  (params (DeltaSeconds :type "Float (single-precision)"))
  (bind (_returnvalue_roll _returnvalue_pitch _returnvalue_yaw) (`KismetMathLibrary.BreakRotator` (`self.K2_GetActorRotation`)))
  (bind (_returnvalue_roll_2 _returnvalue_pitch_2 _returnvalue_yaw_2) (`KismetMathLibrary.BreakRotator` (`self.K2_GetActorRotation`)))
  (bind _returnvalue (`self.GetInputAxisValue`))
  (bind _returnvalue_2 (`self.GetInputAxisValue`))
  (bind _returnvalue_3 (`self.GetInputAxisValue`))
  (bind _plane (`self.plane`))
  (bind _sc_enginesound (`self.SC_EngineSound`))
  (bind _frontlight_intensity (`self.FrontLight Intensity`))
  (bind _sc_doors (`self.SC_Doors`))
  (bind _sc_doors_2 (`self.SC_Doors`))
  (bind _sc_doors_3 (`self.SC_Doors`))
  (bind _sc_doors_4 (`self.SC_Doors`))
  (bind _handbrake (`self.Handbrake`))
  (bind _returnvalue_4 (`KismetMathLibrary.Conv_BoolToDouble` _handbrake))
  (bind (_returnvalue_x _returnvalue_y _returnvalue_z) (`KismetMathLibrary.BreakVector` (`SceneComponent.K2_GetComponentLocation` _plane)))
  (bind _returnvalue_5 (`KismetMathLibrary.Conv_BoolToDouble` (`self.Frontlights`)))
  (bind _returnvalue_6 (`KismetMathLibrary.Abs` (`KismetMathLibrary.VSize` (`self.GetVelocity`))))
  (bind _returnvalue_7 (* (`KismetMathLibrary.Conv_BoolToDouble` (`self.Handbrake`)) (`self.GetInputAxisValue`)))
  (bind (_returnvalue_roll_3 _returnvalue_pitch_3) (`KismetMathLibrary.BreakRotator` (`KismetMathLibrary.MakeRotator` (+ (* _returnvalue_2 10.0) (* _returnvalue_7 15.0)) (* _returnvalue_2 30.0))))
  (bind (_returnvalue_roll_4 _returnvalue_pitch_4 _returnvalue_yaw_3) (`KismetMathLibrary.BreakRotator` (`KismetMathLibrary.RInterpTo` (`KismetMathLibrary.MakeRotator` _returnvalue_roll _returnvalue_pitch _returnvalue_yaw) (`KismetMathLibrary.MakeRotator` _returnvalue_roll_3 _returnvalue_pitch_3 (+ _returnvalue_yaw (* (* (`KismetMathLibrary.SelectFloat` -1.0 1.0 (== _returnvalue_7 -1.0)) (`self.GetInputAxisValue`)) (`self.Rotation Speed`)))) (`self.Delta seconds`) 1.0)))
  (bind _output_get (set `self.Speed` (`KismetMathLibrary.FInterpTo` (`self.Speed`) (* (* (`self.GetInputAxisValue`) _returnvalue_4) (`self.Forward Speed`) 0.05) (`self.Delta seconds`) 1.0)))
  (`PrimitiveComponent.SetEnableGravity` _plane (not (> _returnvalue_z 400.0)))
  (set `self.Delta seconds` DeltaSeconds)
  (`PrimitiveComponent.SetPhysicsLinearVelocity` (`self.plane`) (+ (`self.GetVelocity`) (* (* (`KismetMathLibrary.GreaterGreater_VectorRotator` (`KismetMathLibrary.MakeVector` (* (* (`self.GetInputAxisValue`) _returnvalue_4) (`self.Steer Push`) -0.05) (`KismetMathLibrary.SelectFloat` _output_get 0.0 _handbrake) (`KismetMathLibrary.SelectFloat` (* _returnvalue_4 _returnvalue) (* _returnvalue_4 _returnvalue 5.0) (== _returnvalue -1.0))) (`KismetMathLibrary.MakeRotator` 0.0 0.0 _returnvalue_yaw_2)) (`self.Movement speed`)) (`self.Delta seconds`))) false "None")
  (`self.K2_SetActorRotation` (`KismetMathLibrary.MakeRotator` _returnvalue_roll_4 _returnvalue_pitch_4 _returnvalue_yaw_3)) ; Rotate the helicopter yaw to match the camera, while pitch and roll are determined by input direction
  (bind _output_get_2 (set `self.HoverL` (`KismetMathLibrary.FInterpTo` (`self.HoverL`) (* (`KismetMathLibrary.SelectFloat` _returnvalue_3 0.0 (== _returnvalue_3 1.0)) -18.0) (`GameplayStatics.GetWorldDeltaSeconds`) 2.5)))
  (bind _output_get_3 (set `self.HoverForward` (`KismetMathLibrary.FInterpTo` (`self.HoverForward`) (* (* (`KismetMathLibrary.Conv_BoolToDouble` (`self.Handbrake`)) (`self.GetInputAxisValue`)) 10.0) (`GameplayStatics.GetWorldDeltaSeconds`) 2.5)))
  (bind _returnvalue_8 (+ _output_get_3 10.0))
  (`SceneComponent.K2_SetRelativeRotation` (`self.LeftHover`) (`KismetMathLibrary.MakeRotator` _returnvalue_8 _output_get_2) false false)
  (bind _output_get_4 (set `self.HoverR` (`KismetMathLibrary.FInterpTo` (`self.HoverR`) (* (`KismetMathLibrary.SelectFloat` _returnvalue_3 0.0 (== _returnvalue_3 -1.0)) -18.0) (`GameplayStatics.GetWorldDeltaSeconds`) 2.5)))
  (`SceneComponent.K2_SetRelativeRotation` (`self.RightHover`) (`KismetMathLibrary.MakeRotator` _returnvalue_8 _output_get_4) false false)
  (bind _output_get_5 (set `self.DoorRotFL` (`KismetMathLibrary.FInterpTo` (`self.DoorRotFL`) (`KismetMathLibrary.SelectFloat` 70.0 0.0 (`self.DoorFLOpen?`)) (`GameplayStatics.GetWorldDeltaSeconds`) 5.0)))
  (`SceneComponent.K2_SetRelativeRotation` (`self.FLDoor`) (`KismetMathLibrary.MakeRotator` 0.0 _output_get_5) false false)
  (`AudioComponent.SetFloatParameter` _sc_doors "FLRot" _output_get_5)
  (`AudioComponent.SetBoolParameter` _sc_doors "DoorFL" (`self.DoorFLOpen?`))
  (bind _output_get_6 (set `self.DoorRotFR` (`KismetMathLibrary.FInterpTo` (`self.DoorRotFR`) (`KismetMathLibrary.SelectFloat` -70.0 0.0 (`self.DoorFROpen?`)) (`GameplayStatics.GetWorldDeltaSeconds`) 5.0)))
  (`SceneComponent.K2_SetRelativeRotation` (`self.FRDoor`) (`KismetMathLibrary.MakeRotator` 0.0 _output_get_6) false false)
  (`AudioComponent.SetFloatParameter` _sc_doors_2 "FRRot" _output_get_6)
  (`AudioComponent.SetBoolParameter` _sc_doors_2 "DoorFR" (`self.DoorFROpen?`))
  (bind _output_get_7 (set `self.DoorRotRL` (`KismetMathLibrary.FInterpTo` (`self.DoorRotRL`) (`KismetMathLibrary.SelectFloat` 71.0 0.0 (`self.DoorRLOpen?`)) (`GameplayStatics.GetWorldDeltaSeconds`) 5.0)))
  (`SceneComponent.K2_SetRelativeRotation` (`self.RLDoor`) (`KismetMathLibrary.MakeRotator` -2.384431 _output_get_7) false false)
  (`AudioComponent.SetFloatParameter` _sc_doors_3 "RLRot" _output_get_7)
  (`AudioComponent.SetBoolParameter` _sc_doors_3 "DoorRL" (`self.DoorRLOpen?`))
  (bind _output_get_8 (set `self.DoorRotRR` (`KismetMathLibrary.FInterpTo` (`self.DoorRotRR`) (`KismetMathLibrary.SelectFloat` -71.0 0.0 (`self.DoorRROpen?`)) (`GameplayStatics.GetWorldDeltaSeconds`) 5.0)))
  (`SceneComponent.K2_SetRelativeRotation` (`self.RRDoor`) (`KismetMathLibrary.MakeRotator` -2.384431 _output_get_8) false false)
  (`AudioComponent.SetFloatParameter` _sc_doors_4 "RRRot" _output_get_8)
  (`AudioComponent.SetBoolParameter` _sc_doors_4 "DoorRR" (`self.DoorFROpen?`))
  (bind _output_get_9 (set `self.SteeringWheelRot` (`KismetMathLibrary.FInterpTo` (`self.SteeringWheelRot`) (* (`self.GetInputAxisValue`) 55.0) (`GameplayStatics.GetWorldDeltaSeconds`) 5.0)))
  (`SceneComponent.K2_SetRelativeRotation` (`self.SteeringWheel`) (`KismetMathLibrary.MakeRotator` 0.0 _output_get_9) false false)
  (if (or (== (`self.Handbrake`) false) (== (`self.GetInputAxisValue`) -1.0))
    (set `self.stoplights` 300.0)
    (else
      (set `self.stoplights` 0.0)))
  (`LightComponent.SetIntensity` (`self.Stoplight6`) (`self.stoplights`))
  (`LightComponent.SetIntensity` (`self.Stoplight1`) (`self.stoplights`))
  (`LightComponent.SetIntensity` (`self.Stoplight2`) (`self.stoplights`))
  (`LightComponent.SetIntensity` (`self.Stoplight3`) (`self.stoplights`))
  (`LightComponent.SetIntensity` (`self.Stoplight4`) (`self.stoplights`))
  (`LightComponent.SetIntensity` (`self.Stoplight5`) (`self.stoplights`))
  (`LightComponent.SetIntensity` (`self.Frontlight1`) (* _returnvalue_5 _frontlight_intensity))
  (`LightComponent.SetIntensity` (`self.Frontlight2`) (* _returnvalue_5 _frontlight_intensity))
  (`LightComponent.SetIntensity` (`self.Frontlight3`) (* _returnvalue_5 _frontlight_intensity))
  (`LightComponent.SetIntensity` (`self.PointLight`) (* _returnvalue_5 _frontlight_intensity))
  (`LightComponent.SetIntensity` (`self.FrontSpotLight2`) (* _returnvalue_5 (* _frontlight_intensity 200.0)))
  (`LightComponent.SetIntensity` (`self.FrontSpotLight1`) (* _returnvalue_5 (* _frontlight_intensity 200.0)))
  (`AudioComponent.SetFloatParameter` _sc_enginesound "RPM" _returnvalue_6)
  (`AudioComponent.SetPitchMultiplier` _sc_enginesound (* (+ (/ _returnvalue_6 9000.0) 0.2) 3.0)))

(event `InputAxis|LookUp`
  (params (AxisValue :type "Float (single-precision)"))
  (`SceneComponent.K2_AddRelativeRotation` (`self.SpringArm`) (`KismetMathLibrary.MakeRotator` 0.0 AxisValue (stale `InputAxis|LookRight` AxisValue)) false false :!label _label))

(event `InputAxis|LookRight`
  (params (AxisValue :type "Float (single-precision)"))
  (goto _label))

(event `Key|F`
  (params (Key :type "Key Structure"))
  (:`Pressed`
    (bind _isa (`/Engine/EditorBlueprintResources/StandardMacros.FlipFlop`)
      (:`A`
        _)
      (:`B`
        _))
    (set `self.DoorFLOpen?` _isa)))

(event `Key|T`
  (params (Key :type "Key Structure"))
  (:`Pressed`
    (bind _isa (`/Engine/EditorBlueprintResources/StandardMacros.FlipFlop`)
      (:`A`
        _)
      (:`B`
        _))
    (set `self.Frontlights` _isa)))

(event `Key|R`
  (params (Key :type "Key Structure"))
  (:`Pressed`
    (bind _isa (`/Engine/EditorBlueprintResources/StandardMacros.FlipFlop`)
      (:`A`
        _)
      (:`B`
        _))
    (set `self.DoorFROpen?` _isa)))

(event `Key|Z`
  (params (Key :type "Key Structure"))
  (:`Pressed`
    (bind _isa (`/Engine/EditorBlueprintResources/StandardMacros.FlipFlop`)
      (:`A`
        _)
      (:`B`
        _))
    (set `self.DoorRLOpen?` _isa)))

(event `Key|X`
  (params (Key :type "Key Structure"))
  (:`Pressed`
    (bind _isa (`/Engine/EditorBlueprintResources/StandardMacros.FlipFlop`)
      (:`A`
        _)
      (:`B`
        _))
    (set `self.DoorRROpen?` _isa)))

(event `Key|SpaceBar`
  (params (Key :type "Key Structure"))
  (:`Pressed`
    (set `self.Handbrake` false))
  (:`Released`
    (set `self.Handbrake` true)))

(fn `UserConstructionScript`
  (bind _body (`self.Body`))
  (`MeshComponent.SetVectorParameterValueOnMaterials` _body "Param" (`KismetMathLibrary.Conv_LinearColorToVector` (`self.BodyColor`)))
  (`MeshComponent.SetVectorParameterValueOnMaterials` (`self.LeftHover`) "Param" (`KismetMathLibrary.Conv_LinearColorToVector` (`self.BodyColor`)))
  (`MeshComponent.SetVectorParameterValueOnMaterials` (`self.RightHover`) "Param" (`KismetMathLibrary.Conv_LinearColorToVector` (`self.BodyColor`)))
  (`MeshComponent.SetVectorParameterValueOnMaterials` (`self.FLDoor`) "Param" (`KismetMathLibrary.Conv_LinearColorToVector` (`self.BodyColor`)))
  (`MeshComponent.SetVectorParameterValueOnMaterials` (`self.RLDoor`) "Param" (`KismetMathLibrary.Conv_LinearColorToVector` (`self.BodyColor`)))
  (`MeshComponent.SetVectorParameterValueOnMaterials` (`self.RRDoor`) "Param" (`KismetMathLibrary.Conv_LinearColorToVector` (`self.BodyColor`)))
  (`MeshComponent.SetVectorParameterValueOnMaterials` (`self.FRDoor`) "Param" (`KismetMathLibrary.Conv_LinearColorToVector` (`self.BodyColor`)))
  (`MeshComponent.SetScalarParameterValueOnMaterials` _body "Dirt Level" (`self.Dirt Level`))
  (`MeshComponent.SetScalarParameterValueOnMaterials` (`self.FRDoor`) "Dirt Level" (`self.Dirt Level`))
  (`MeshComponent.SetScalarParameterValueOnMaterials` (`self.RRDoor`) "Dirt Level" (`self.Dirt Level`))
  (`MeshComponent.SetScalarParameterValueOnMaterials` (`self.RLDoor`) "Dirt Level" (`self.Dirt Level`))
  (`MeshComponent.SetScalarParameterValueOnMaterials` (`self.FLDoor`) "Dirt Level" (`self.Dirt Level`))
  (`MeshComponent.SetScalarParameterValueOnMaterials` (`self.LeftHover`) "Dirt Level" (`self.Dirt Level`))
  (`MeshComponent.SetScalarParameterValueOnMaterials` (`self.RightHover`) "Dirt Level" (`self.Dirt Level`))
  (`LightComponent.SetLightColor` (`self.FrontSpotLight2`) (`self.Frontlight`) true)
  (`LightComponent.SetLightColor` (`self.Frontlight2`) (`self.Frontlight`) true)
  (`LightComponent.SetLightColor` (`self.FrontSpotLight1`) (`self.Frontlight`) true)
  (`LightComponent.SetLightColor` (`self.Frontlight3`) (`self.Frontlight`) true)
  (`LightComponent.SetLightColor` (`self.PointLight`) (`self.Frontlight`) true)
  (`LightComponent.SetLightColor` (`self.Frontlight1`) (`self.Frontlight`) true))