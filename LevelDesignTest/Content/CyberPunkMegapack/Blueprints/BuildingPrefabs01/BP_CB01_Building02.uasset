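; BP_CB01_Building02 is a cyberpunk building prefab made of static mesh modules with configurable billboards.
; The construction script assigns four billboard material variables (big, small and two ground-level) to named material slots on four of the mesh components.
; It has no active runtime logic, as the event graph holds only disabled placeholder events.
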(fn `UserConstructionScript`
  (`PrimitiveComponent.SetMaterialByName` (`self.SM_CPB7_Module14`) "BillboardBig" (`self.Big Billboard`))
  (`PrimitiveComponent.SetMaterialByName` (`self.SM_CPB7_Module07`) "BillboardSmall" (`self.BillboardSmall`))
  (`PrimitiveComponent.SetMaterialByName` (`self.SM_CPB7_Module01`) "Billboard" (`self.Billboard Ground 01`))
  (`PrimitiveComponent.SetMaterialByName` (`self.StaticMesh`) "Billboard" (`self.Billboard Ground 02`)))