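; Fountain actor Blueprint that tints its Niagara water effect with a configurable Color.
; Creates a dynamic instance of the M_Splash_Refract material, sets its Color vector parameter, and passes it to NSFountain as the Niagara material variable, also named Color.
; The same setup runs in the Construction Script and again on BeginPlay, so the tint applies at construction and at runtime.
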(event `self.ReceiveBeginPlay`
  (bind _returnvalue (`KismetMaterialLibrary.CreateDynamicMaterialInstance` "/Game/A_Surface_Footstep/Niagara_FX/Materials/M_Splash_Refract.M_Splash_Refract"))
  (bind _output_get (set `self.Matrial Dynamic` _returnvalue))
  (`MaterialInstanceDynamic.SetVectorParameterValue` _output_get "Color" (`self.Color`))
  (`NiagaraComponent.SetVariableMaterial` (`self.NS_Fountain`) "Color" (`self.Matrial Dynamic`)))

(fn `UserConstructionScript`
  (bind _returnvalue (`KismetMaterialLibrary.CreateDynamicMaterialInstance` "/Game/A_Surface_Footstep/Niagara_FX/Materials/M_Splash_Refract.M_Splash_Refract"))
  (bind _output_get (set `self.Matrial Dynamic` _returnvalue))
  (`MaterialInstanceDynamic.SetVectorParameterValue` _output_get "Color" (`self.Color`))
  (`NiagaraComponent.SetVariableMaterial` (`self.NS_Fountain`) "Color" (`self.Matrial Dynamic`)))