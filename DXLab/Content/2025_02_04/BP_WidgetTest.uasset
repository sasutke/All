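; BP_WidgetTest is a test actor with a widget component that stays hidden until shown.
; BeginPlay hides the widget, and the ShowUI and HideUI functions toggle its visibility.
; Each Tick billboards the widget toward the player camera on yaw only, using a look-at rotation from camera to actor flipped 180 degrees so it stays upright.
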(event `self.ReceiveBeginPlay`
  (`SceneComponent.SetVisibility` (`self.Widget`) false false))

(event `self.ReceiveTick`
  (params (DeltaSeconds :type "Float (single-precision)"))
  (`SceneComponent.K2_SetWorldRotation` (`self.Widget`) (`KismetMathLibrary.MakeRotator` 0.0 0.0 (+ (.yaw (`KismetMathLibrary.FindLookAtRotation` (`PlayerCameraManager.GetCameraLocation` (`GameplayStatics.GetPlayerCameraManager` 0)) (`self.K2_GetActorLocation`))) 180.0)) false false))

(fn `HideUI`
  (`SceneComponent.SetVisibility` (`self.Widget`) false false))

(fn `ShowUI`
  (`SceneComponent.SetVisibility` (`self.Widget`) true false))

(fn `UserConstructionScript`)