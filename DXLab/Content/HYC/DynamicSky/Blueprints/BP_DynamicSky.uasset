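; Dynamic sky actor that sets up a day/night sky from a time-of-day value, entirely in the Construction Script with no runtime update.
; It creates a dynamic sky sphere material, maps time against dawn and dusk to sun and moon light pitch, and toggles their visibility.
; At night it applies moonlight, atmosphere scattering and star/moon material settings; by day it restores fixed scattering and hides stars and moon.
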(fn `Handle Sun Moon Rotation`
  ; sun rotation between dawn and dusk
  (`SceneComponent.K2_SetWorldRotation` (`self.SunDirectionalLight`) (`KismetMathLibrary.MakeRotator` 0.0 (`KismetMathLibrary.MapRangeUnclamped` (`self.TimeofDay`) (`self.Dawn Time`) (`self.Dusk Time`) 0.0 -180.0)) false false)
  ; moon rotation after dusk
  (`SceneComponent.K2_SetWorldRotation` (`self.MoonDirectionalLight`) (`KismetMathLibrary.MakeRotator` 0.0 (`KismetMathLibrary.MapRangeUnclamped` (`self.TimeofDay`) (+ (`self.Dusk Time`) 0.3) 24.0 -180.0 -90.0)) false false)
  ; moon rotation before dawn
  (`SceneComponent.K2_SetWorldRotation` (`self.MoonDirectionalLight`) (`KismetMathLibrary.MakeRotator` 0.0 (`KismetMathLibrary.MapRangeUnclamped` (`self.TimeofDay`) 0.0 (- (`self.Dawn Time`) 0.2) -90.0)) false false))

(fn `HandleNightSettings`
  (if (`self.Is NightTime`)
    (`|ExecutionSequence`
      (:`then_0`
        (`LightComponent.SetIntensity` (`self.MoonDirectionalLight`) (`self.Moonlight Intensity`))
        (`LightComponent.SetLightColor` (`self.MoonDirectionalLight`) (`self.MoonLight Color`) true)
        (`DirectionalLightComponent.SetLightSourceAngle` (`self.MoonDirectionalLight`) (`self.MoonLight SourceAngle`))
        (`LightComponent.SetTemperature` (`self.MoonDirectionalLight`) (`self.MoonLight Temperature`)))
      (:`then_1`
        (`SkyAtmosphereComponent.SetRayleighScattering` (`self.SkyAtmosphere`) (`self.Nighttime Rayleigh Scattering`))
        (`SkyAtmosphereComponent.SetMultiScatteringFactor` (`self.SkyAtmosphere`) (`self.Nighttime Multi Scattering`)))
      (:`then_2`
        (`MaterialInstanceDynamic.SetScalarParameterValue` (`self.Created_DynMI_SkySphere`) "IsStarVisible" (`KismetMathLibrary.SelectFloat` 1.0 0.0 (`self.ShouldShowStars`)))
        (`MaterialInstanceDynamic.SetScalarParameterValue` (`self.Created_DynMI_SkySphere`) "IsMoonVisible" (`KismetMathLibrary.SelectFloat` 1.0 0.0 (`self.Should Show Moon`)))
        (`MaterialInstanceDynamic.SetVectorParameterValue` (`self.Created_DynMI_SkySphere`) "MoonBasicSettings" (make `LinearColor` (/ (`self.MoonScale`) 10.0) (`self.MoonStaticRotation`) (`self.MoonBrightness`) 1.0))
        (`MaterialInstanceDynamic.SetVectorParameterValue` (`self.Created_DynMI_SkySphere`) "MoonTint" (`self.MoonTint`))))
    (else
      (`SkyAtmosphereComponent.SetRayleighScattering` (`self.SkyAtmosphere`) (struct :`R` 0.174647 :`G` 0.40724 :`B` 1.0 :`A` 1.0))
      (`SkyAtmosphereComponent.SetMultiScatteringFactor` (`self.SkyAtmosphere`) 1.0)
      (`MaterialInstanceDynamic.SetScalarParameterValue` (`self.Created_DynMI_SkySphere`) "IsStarVisible" 0.0)
      (`MaterialInstanceDynamic.SetScalarParameterValue` (`self.Created_DynMI_SkySphere`) "IsMoonVisible" 0.0))))

(fn `HandleVisibility`
  (`SceneComponent.SetVisibility` (`self.SunDirectionalLight`) (`self.Is DayTime`) false)
  (`SceneComponent.SetVisibility` (`self.MoonDirectionalLight`) (`self.Is NightTime`) false))

(fn `InitSkySphereMaterial`
  (returns (Is_DynMI_SkySphereValid :type Boolean))
  (bind _returnvalue (`PrimitiveComponent.CreateDynamicMaterialInstance` (`self.SM_Sky Sphere`) 0 "/Game/HYC/DynamicSky/Materials/Sky/MI_DynamicSkySphere.MI_DynamicSkySphere" "None"))
  (bind _output_get (set `self.Created_DynMI_SkySphere` _returnvalue))
  (return (`KismetSystemLibrary.IsValid` _output_get)))

(fn `UserConstructionScript`
  (bind _is_dynmi_skyspherevalid (`self.InitSkySphereMaterial`))
  (if _is_dynmi_skyspherevalid
    (`|ExecutionSequence`
      (:`then_1`
        (`self.Handle Sun Moon Rotation`))
      (:`then_2`
        (`self.HandleVisibility`))
      (:`then_3`
        (`self.HandleNightSettings`)))))